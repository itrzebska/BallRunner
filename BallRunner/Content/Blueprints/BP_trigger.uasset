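; BP_trigger is a box trigger that is set up to restart the current level when the player pawn overlaps it.
; On overlap it destroys itself, then starts a held camera fade-out and a matching Delay, followed by reopening the level by name and calling a fade-in.
; The self-destruction precedes the latent Delay, so the reload and fade-in depend on a timer owned by a destroyed actor.
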(event OnComponentBeginOverlap(Box)
  (params (OverlappedComponent :type Primitive%20Component%20Object%20Reference) (OtherActor :type Actor%20Object%20Reference) (OtherComp :type Primitive%20Component%20Object%20Reference) (OtherBodyIndex :type Integer) (bFromSweep :type Boolean) (SweepResult :type Hit%20Result%20Structure%20%28by%20ref%29))
  (if (== (Game|Player|GetPlayerPawn 0) OtherActor)
    (Actor|DestroyActor)
    (CameraFades|StartCameraFade :self (Game|GetPlayerCameraManager 0) :ToAlpha 1.0 :Duration 2.0 :bHoldWhenFinished true)
    (Utilities|FlowControl|Delay 2.0)
    (bind _returnvalue (Game|GetCurrentLevelName true))
    (Game|OpenLevel(byName) (Utilities|String|StringToName _returnvalue))
    (CameraFades|StartCameraFade :self (Game|GetPlayerCameraManager 0) :FromAlpha 1.0 :ToAlpha 0.0 :Duration 1.5 :bHoldWhenFinished true)))

(fn ConstructionScript)